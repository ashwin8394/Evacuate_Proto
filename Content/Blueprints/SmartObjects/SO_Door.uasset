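; Smart-object double door that swings open and closed, either with the Use input or automatically when the player is near.
; A trigger sets InRange, and Tick checks it against the door settings for locking, key interaction and auto-close.
; Gates and cross-resetting DoOnce nodes drive four timelines that lerp between start and end rotations.
; RotateDoor mirrors the left leaf's yaw from the right, and the construction script previews meshes and open state.
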(event `self.ReceiveBeginPlay`
  (`self.EnableInput` (`GameplayStatics.GetPlayerController` 0)))

(event `self.Trigger.OnComponentBeginOverlap`
  (params (OverlappedComponent :type "PrimitiveComponent Object Reference") (OtherActor :type "Actor Object Reference") (OtherComp :type "PrimitiveComponent Object Reference") (OtherBodyIndex :type Integer) (bFromSweep :type Boolean) (SweepResult :type "HitResult Structure (by ref)"))
  (if (== OtherActor (`GameplayStatics.GetPlayerPawn` 0))
    (set `self.inRange` true)
    (else
      (set `self.inRange` false))))

(event `self.Trigger.OnComponentEndOverlap`
  (params (OverlappedComponent :type "PrimitiveComponent Object Reference") (OtherActor :type "Actor Object Reference") (OtherComp :type "PrimitiveComponent Object Reference") (OtherBodyIndex :type Integer))
  (if (== OtherActor (`GameplayStatics.GetPlayerPawn` 0))
    _
    (else
      _))
  (set `self.inRange` false))

(event `InputAction|Use` :consume false :overrideparent false
  (params (Key :type "Key Structure" :default "AnyKey"))
  (bind _doorsettings (`self.DoorSettings`))
  (bind _doorsettings_2 (`self.DoorSettings`))
  (bind _doorsettings_3 (`self.DoorSettings`))
  (bind _doorsettings_4 (`self.DoorSettings`))
  ;[1 1 1] Close door with key action
  (:`Pressed`
    (goto _label :!via `Open`))
  (:`Released`
    (goto _label :!via `Close`)))

(event `self.ReceiveTick`
  (params (DeltaSeconds :type "Float (single-precision)"))
  (bind (_doorsettings_locked _doorsettings_autoclose _doorsettings_interactwithkey) (break `/Game/Blueprints/DataTypes/Door` (`self.DoorSettings`)))
  (bind (_doorsettings_locked_2 _doorsettings_autoclose_2) (break `/Game/Blueprints/DataTypes/Door` (`self.DoorSettings`)))
  (bind _doorsettings (`self.DoorSettings`))
  (bind _doorsettings_2 (`self.DoorSettings`))
  (bind _doorsettings_3 (`self.DoorSettings`))
  (bind _doorsettings_4 (`self.DoorSettings`))
  ;[1 1 1] Check door position
  (if (and (`self.inRange`) (not _doorsettings_locked_2))
    (if (`self.Open`)
      ;[1 1 1] Close door with key action
      (if _doorsettings_interactwithkey
        (`/Engine/EditorBlueprintResources/StandardMacros.Gate` true :!label _label
          (:`Exit`
            (`/Engine/EditorBlueprintResources/StandardMacros.DoOnce` false :!label _label_2
              (:`Completed`
                (bind (_direction _dooranim) (`Timeline|SwingClosed` :!via `PlayFromStart`)
                  (:`Update`
                    (`self.RotateDoor` (`KismetMathLibrary.RLerp` (.rotation (`.EndPosition_11_1D88593546FA91DADE03E2BD5AB37CC9` (break `/Game/Blueprints/DataTypes/Door` _doorsettings_2))) (.rotation (`.StartPosition_8_7C3F542A41233467D869988DFEB1F7CD` (break `/Game/Blueprints/DataTypes/Door` _doorsettings_2))) _dooranim)))
                  (:`Finished`
                    (set `self.Open` false)
                    (`|ExecutionSequence`
                      (:`then_0`
                        (goto _label_4 :!via `Reset`))
                      (:`then_1`
                        (goto _label_5 :!via `Reset`))))))))))
      (else
        ;[1 1 1] Open door with key action
        (if _doorsettings_interactwithkey
          (`/Engine/EditorBlueprintResources/StandardMacros.Gate` true :!label _label_3
            (:`Exit`
              (`/Engine/EditorBlueprintResources/StandardMacros.DoOnce` false :!label _label_4
                (:`Completed`
                  (bind (_direction_2 _dooranim_2) (`Timeline|SwingOpen` :!via `PlayFromStart`)
                    (:`Update`
                      (`self.RotateDoor` (`KismetMathLibrary.RLerp` (.rotation (`.StartPosition_8_7C3F542A41233467D869988DFEB1F7CD` (break `/Game/Blueprints/DataTypes/Door` _doorsettings_3))) (.rotation (`.EndPosition_11_1D88593546FA91DADE03E2BD5AB37CC9` (break `/Game/Blueprints/DataTypes/Door` _doorsettings_3))) _dooranim_2 true)))
                    (:`Finished`
                      (set `self.Open` true)
                      (`|ExecutionSequence`
                        (:`then_0`
                          (goto _label_2 :!via `Reset`))
                        (:`then_1`
                          (goto _label_6 :!via `Reset`)))))))))
          (else
            ;[1 1 1] Open Door When Near
            (`/Engine/EditorBlueprintResources/StandardMacros.DoOnce` false :!label _label_5
              (:`Completed`
                (bind (_direction_3 _dooranim_3) (`Timeline|SwingOpenAuto` :!via `PlayFromStart`)
                  (:`Update`
                    (`self.RotateDoor` (`KismetMathLibrary.RLerp` (.rotation (`.StartPosition_8_7C3F542A41233467D869988DFEB1F7CD` (break `/Game/Blueprints/DataTypes/Door` _doorsettings_4))) (.rotation (`.EndPosition_11_1D88593546FA91DADE03E2BD5AB37CC9` (break `/Game/Blueprints/DataTypes/Door` _doorsettings_4))) _dooranim_3 true)))
                  (:`Finished`
                    (set `self.Open` true)
                    (`|ExecutionSequence`
                      (:`then_0`
                        (goto _label_6 :!via `Reset`))
                      (:`then_1`
                        (goto _label_2 :!via `Reset`)))))))))))
    (else
      ;[1 1 1] Close Door when out of range
      (if (and (`KismetMathLibrary.BooleanNOR` _doorsettings_locked_2 (`self.inRange`)) _doorsettings_autoclose_2 (`self.Open`))
        (`/Engine/EditorBlueprintResources/StandardMacros.DoOnce` false :!label _label_6
          (:`Completed`
            (bind (_direction_4 _dooranim_4) (`Timeline|SwingCloseAuto` :!via `PlayFromStart`)
              (:`Update`
                (`self.RotateDoor` (`KismetMathLibrary.RLerp` (.rotation (`.EndPosition_11_1D88593546FA91DADE03E2BD5AB37CC9` (break `/Game/Blueprints/DataTypes/Door` _doorsettings))) (.rotation (`.StartPosition_8_7C3F542A41233467D869988DFEB1F7CD` (break `/Game/Blueprints/DataTypes/Door` _doorsettings))) _dooranim_4)))
              (:`Finished`
                (set `self.Open` false)
                (`|ExecutionSequence`
                  (:`then_0`
                    (goto _label_5 :!via `Reset`))
                  (:`then_1`
                    (goto _label_4 :!via `Reset`)))))))))))

(event `InputAction|Use` :consume false :overrideparent false
  (params (Key :type "Key Structure" :default "AnyKey"))
  ;[1 1 1] Open door with key action
  (:`Pressed`
    (goto _label_3 :!via `Open`))
  (:`Released`
    (goto _label_3 :!via `Close`)))

(fn `leftDoorCoordinate`
  (params (RightDoorTargetRotation :type "Rotator Structure") (offset :type "Rotator Structure"))
  (returns (out :type "Rotator Structure"))
  (return (`KismetMathLibrary.MakeRotator` (.roll RightDoorTargetRotation) (.pitch RightDoorTargetRotation) (- (.yaw offset) (.yaw RightDoorTargetRotation)))))

(fn `RotateDoor`
  (params (TargetRotation :type "Rotator Structure"))
  (bind (_rightdooroffset_location _rightdooroffset_rotation) (`KismetMathLibrary.BreakTransform` (`self.RightDoorOffset`)))
  (bind (_leftdooroffest_location _leftdooroffest_rotation) (`KismetMathLibrary.BreakTransform` (`self.LeftDoorOffest`)))
  (bind _returnvalue (`KismetMathLibrary.ComposeRotators` TargetRotation _rightdooroffset_rotation))
  (`SceneComponent.K2_SetRelativeRotation` (`self.RightDoor`) _returnvalue false false)
  (bind _out (`self.leftDoorCoordinate` _returnvalue _leftdooroffest_rotation))
  (`SceneComponent.K2_SetRelativeRotation` (`self.LeftDoor`) _out false false)
  (return))

(fn `UserConstructionScript`
  (bind _doorsettings (`self.DoorSettings`))
  (`StaticMeshComponent.SetStaticMesh` (`self.LeftDoor`) (`self.LeftDoorMesh`))
  (`StaticMeshComponent.SetStaticMesh` (`self.RightDoor`) (`self.RightDoorMesh`))
  (`SceneComponent.K2_AddLocalTransform` (`self.LeftDoor`) (`self.LeftDoorOffest`) false false)
  (`SceneComponent.K2_AddLocalTransform` (`self.RightDoor`) (`self.RightDoorOffset`) false false)
  (if (`self.Open`)
    (`self.RotateDoor` (.rotation (`.EndPosition_11_1D88593546FA91DADE03E2BD5AB37CC9` (break `/Game/Blueprints/DataTypes/Door` _doorsettings))))
    (else
      (`self.RotateDoor` (.rotation (`.StartPosition_8_7C3F542A41233467D869988DFEB1F7CD` (break `/Game/Blueprints/DataTypes/Door` _doorsettings)))))))