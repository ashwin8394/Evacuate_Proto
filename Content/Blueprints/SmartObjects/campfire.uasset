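; Campfire smart object that toggles its fire and light and alters the level's height fog around it.
; Tick and the construction script apply the Active flag to both effects; on Tick, EmitOnly also keeps the fire running without the light.
; Overlapping FogBurnZone reverses a timeline and leaving plays it forward, scaling the first found ExponentialHeightFog's start distance while Active.
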(event `self.ReceiveBeginPlay`
  (bind _outactors (`GameplayStatics.GetAllActorsOfClass` "/Script/Engine.ExponentialHeightFog"))
  (set `self.Fog_Ref` (`KismetArrayLibrary.Array_Get` _outactors)))

(event `self.ReceiveTick`
  (params (DeltaSeconds :type "Float (single-precision)"))
  (bind _active (`self.Active`))
  (`ActorComponent.SetActive` (`self.Fire`) (or (`self.Emit Only`) _active) false)
  (`SceneComponent.SetVisibility` (`self.PointLight`) _active false))

(event `self.FogBurnZone.OnComponentBeginOverlap`
  (params (OverlappedComponent :type "PrimitiveComponent Object Reference") (OtherActor :type "Actor Object Reference") (OtherComp :type "PrimitiveComponent Object Reference") (OtherBodyIndex :type Integer) (bFromSweep :type Boolean) (SweepResult :type "HitResult Structure (by ref)"))
  (bind (_direction _transition) (`Timeline|FogStartDist` :!via `Reverse` :!label _label)
    (:`Update`
      (if (`self.Active`)
        (`ExponentialHeightFogComponent.SetStartDistance` (`ExponentialHeightFog.Component` (`self.Fog_Ref`)) (* _transition 300.0))))))

(event `self.FogBurnZone.OnComponentEndOverlap`
  (params (OverlappedComponent :type "PrimitiveComponent Object Reference") (OtherActor :type "Actor Object Reference") (OtherComp :type "PrimitiveComponent Object Reference") (OtherBodyIndex :type Integer))
  (goto _label))

(fn `UserConstructionScript`
  (bind _active (`self.Active`))
  (`ActorComponent.SetActive` (`self.Fire`) _active false)
  (`SceneComponent.SetVisibility` (`self.PointLight`) _active false))