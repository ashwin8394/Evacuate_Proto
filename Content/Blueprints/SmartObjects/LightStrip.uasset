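; Overhead light strip trap that drops its three lights on players or NPCs passing underneath.
; A randomized countdown arms the trigger; overlaps select the nearest still-attached light and roll to drop it, killing its glow, starting sparks and adjusting later odds.
; Fixture fracture or all three falling releases the destructible fixture with radius damage.
; That collapse also sphere-traces downward, electrifying broken WaterPipe actors if the strip is electrically active.
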(event `self.Trigger.OnComponentBeginOverlap`
  (params (OverlappedComponent :type "PrimitiveComponent Object Reference") (OtherActor :type "Actor Object Reference") (OtherComp :type "PrimitiveComponent Object Reference") (OtherBodyIndex :type Integer) (bFromSweep :type Boolean) (SweepResult :type "HitResult Structure (by ref)"))
  (bind _returnvalue (`GameplayStatics.GetObjectClass` OtherActor))
  (bind _returnvalue_2 (`self.K2_GetActorLocation` OtherActor))
  (bind _overhead_light_1 (`self.Overhead_Light_1`))
  (bind _overhead_light2 (`self.Overhead_Light2`))
  (bind _overhead_light_3 (`self.Overhead_Light_3`))
  ;[1 1 1] Overlap Calculation (reduces physics volume count)
  (if (or (== _returnvalue "/Game/Objects/Character/Player_Character2.Player_Character2_C") (== _returnvalue "/Game/Blueprints/Character/AI_Character/NPC.NPC_C"))
    (`|ExecutionSequence`
      (:`then_0`
        (bind _distance (`self.Distance to Initiator` (`SceneComponent.K2_GetComponentLocation` _overhead_light_1) _returnvalue_2 (not (`SceneComponent.IsSimulatingPhysics` _overhead_light_1 "None"))))
        (bind _distance_2 (`self.Distance to Initiator` (`SceneComponent.K2_GetComponentLocation` _overhead_light2) _returnvalue_2 (not (`SceneComponent.IsSimulatingPhysics` _overhead_light2 "None"))))
        (bind _distance_3 (`self.Distance to Initiator` (`SceneComponent.K2_GetComponentLocation` _overhead_light_3) _returnvalue_2 (not (`SceneComponent.IsSimulatingPhysics` _overhead_light_3 "None")))))
      (:`then_1`
        (bind _returnvalue_3 (`KismetMathLibrary.FMin` _distance _distance_2 _distance_3))
        ;[1 1 1] EVENT: Overlap Trigger 1
        (if (== _distance _returnvalue_3)
          (`self.TRAP_Overhead_Falling` (`self.Overhead_Light_1`) (`self.SpotLight1`) (`self.PointLight1`) (`self.Sparks1`))
          (else
            ;[1 1 1] EVENT: Overlap Trigger 2
            (if (== _distance_2 _returnvalue_3)
              (`self.TRAP_Overhead_Falling` (`self.Overhead_Light2`) (`self.SpotLight2`) (`self.PointLight2`) (`self.Sparks2`))
              (else
                ;[1 1 1] EVENT: Overlap Trigger 3
                (if (== _distance_3 _returnvalue_3)
                  (`self.TRAP_Overhead_Falling` (`self.Overhead_Light_3`) (`self.SpotLight3`) (`self.PointLight3`) (`self.Sparks3`))
                  (else
                    (`ActorComponent.Deactivate` (`self.Trigger`))))))))))))

(event `self.ReceiveTick`
  (params (DeltaSeconds :type "Float (single-precision)"))
  (bind _active_timer (`self.Active Timer`))
  (bind _dm_light_fixture (`self.DM_Light_Fixture`))
  (bind _dm_light_fixture_2 (`self.DM_Light_Fixture`))
  (bind _returnvalue (`KismetMathLibrary.VSize` (`SceneComponent.GetComponentVelocity` _dm_light_fixture)))
  ;[1 1 1] Timer until Active
  (`|ExecutionSequence`
    (:`then_0`
      (`/Engine/EditorBlueprintResources/StandardMacros.DoOnce` false :!label _label
        (:`Completed`
          (if (<= _active_timer 0.0)
            (set `PrimitiveComponent.bGenerateOverlapEvents` true (`self.Trigger`))
            (set `self.Active Timer` 0.0)
            (else
              (set `self.Active Timer` (- _active_timer (`KismetMathLibrary.Conv_IntToDouble` (`KismetMathLibrary.FCeil` DeltaSeconds))))
              (goto _label :!via `Reset`))))))
    (:`then_1`
      ;[1 1 1] Trigger all if Fixture fractures and then trace for water on ground
      (`KismetSystemLibrary.Delay` 0.2)
      (if (> _returnvalue 0.0)
        (`KismetSystemLibrary.PrintString` (`KismetStringLibrary.Concat_StrStr` (`KismetSystemLibrary.GetDisplayName` _dm_light_fixture) " = " (`KismetStringLibrary.Conv_DoubleToString` _returnvalue)) true true (struct :`G` 0.66 :`B` 1.0 :`A` 1.0) 0.2))
      (if (and (`SceneComponent.IsSimulatingPhysics` (`self.Overhead_Light_1`) "None") (`SceneComponent.IsSimulatingPhysics` (`self.Overhead_Light2`) "None") (`SceneComponent.IsSimulatingPhysics` (`self.Overhead_Light_3`) "None"))
        (`self.TraceForWaterOnGround` :!label _label_2)
        (`self.TRAP_Overhead_Falling` (`self.Overhead_Light_1`) (`self.SpotLight1`) (`self.PointLight1`) (`self.Sparks1`) true)
        (`self.TRAP_Overhead_Falling` (`self.Overhead_Light2`) (`self.SpotLight2`) (`self.PointLight2`) (`self.Sparks2`) true)
        (`self.TRAP_Overhead_Falling` (`self.Overhead_Light_3`) (`self.SpotLight3`) (`self.PointLight3`) (`self.Sparks3`) true)
        (`ActorComponent.Deactivate` (`self.Trigger`))
        (`PrimitiveComponent.SetSimulatePhysics` _dm_light_fixture_2 true)
        (`DestructibleComponent.ApplyRadiusDamage` _dm_light_fixture_2 100.0 (`SceneComponent.K2_GetComponentLocation` _dm_light_fixture_2) 1000.0 1000.0 true)
        (set `self.DM_Broken` true)))))

(event `self.DM_Light_Fixture.OnComponentFracture`
  (params (HitPoint :type "Vector Structure (by ref)") (HitDirection :type "Vector Structure (by ref)"))
  ;[1 1 1] Trigger all if Fixture fractures and then trace for water on ground
  (goto _label_2))

(fn `Distance to Initiator`
  (params (`Component World Location` :type "Vector Structure") (`Initiator World Location` :type "Vector Structure") (Enable :type Boolean))
  (returns (Distance :type "Float (double-precision)"))
  (if Enable
    (return (`KismetMathLibrary.VSize` (- `Component World Location` `Initiator World Location`)))
    (else
      (return 2147483647.0))))

(fn `TraceForWaterOnGround`
  (bind _returnvalue (`SceneComponent.K2_GetComponentLocation` (`self.DefaultSceneRoot`)))
  (if (`self.DM_Electrically_Active`)
    (bind _outhits (`KismetSystemLibrary.SphereTraceMultiForObjects` _returnvalue (`KismetMathLibrary.MakeVector` (.x _returnvalue) (.y _returnvalue) -10500.0) 4000.0 (`|MakeArray` "ObjectTypeQuery2" "ObjectTypeQuery1" :!type "EObjectTypeQuery Enum")))
    (`/Engine/EditorBlueprintResources/StandardMacros.DoOnce` false :!label _label
      (:`Completed`
        (for _array_element _outhits
          (bind (_bblockinghit _binitialoverlap _time _location _impactpoint _normal _impactnormal _physmat _hitactor) (`GameplayStatics.BreakHitResult` _array_element))
          (if (== (`GameplayStatics.GetObjectClass` _hitactor) "/Game/Blueprints/SmartObjects/WaterPipe.WaterPipe_C")
            (bind _aswater_pipe (cast `/Game/Blueprints/SmartObjects/WaterPipe` _hitactor))
            (if (`/Game/Blueprints/SmartObjects/WaterPipe.Broken` _aswater_pipe)
              (set `/Game/Blueprints/SmartObjects/WaterPipe.Electric` true _aswater_pipe))))
        (set `self.DM_Broken` true)
        (goto _label :!via `Reset`)))))

(fn `TRAP_Overhead_Falling`
  (params (Overhead_Light :type "PrimitiveComponent Object Reference (by ref)") (Spotlight :type "SpotLightComponent Object Reference") (Pointlight :type "PointLightComponent Object Reference") (Sparks :type "ParticleSystemComponent Object Reference") (ForceFall :type Boolean))
  (bind (_trap_active _trap_traptype _trap_activechance _trap_activetime _trap_activerange _trap_maxtriggercount _trap_triggercount _trap_localinfluence) (break `/Game/Blueprints/DataTypes/Environment_Trap` (`self.Trap`)))
  (bind (_trap_active_2 _trap_traptype_2 _trap_activechance_2 _trap_activetime_2 _trap_activerange_2 _trap_maxtriggercount_2 _trap_triggercount_2 _trap_localinfluence_2) (break `/Game/Blueprints/DataTypes/Environment_Trap` (`self.Trap`)))
  (bind _returnvalue (> _trap_maxtriggercount _trap_triggercount))
  ;[1 1 1] If trap has not been activated, activate
  (set `self.Trap` (make `/Game/Blueprints/DataTypes/Environment_Trap` _returnvalue _trap_traptype _trap_activechance _trap_activetime _trap_activerange _trap_maxtriggercount _trap_triggercount _trap_localinfluence))
  ;[1 1 1] If random value is within Active chance bounds
  (if _returnvalue
    (if (or ForceFall (>= _trap_activechance (`KismetMathLibrary.RandomFloatInRange` 0.0 1.0)))
      (`SceneComponent.SetVisibility` Spotlight false false)
      (`ActorComponent.SetActive` Sparks true false)
      ;[1 1 1] Enable Physics: Fall
      (`PrimitiveComponent.SetSimulatePhysics` Overhead_Light true)
      (`SceneComponent.SetVisibility` Pointlight false false)
      ;[1 1 1] Inflict damage radial to Location of Light
      (set `self.Trap` (make `/Game/Blueprints/DataTypes/Environment_Trap` _trap_active_2 _trap_traptype_2 (+ _trap_activechance_2 _trap_localinfluence_2) _trap_activetime_2 _trap_activerange_2 _trap_maxtriggercount_2 (+ (`KismetMathLibrary.Conv_BoolToInt` (`SceneComponent.IsAnySimulatingPhysics` (`self.Overhead_Light_1`))) (`KismetMathLibrary.Conv_BoolToInt` (`SceneComponent.IsAnySimulatingPhysics` (`self.Overhead_Light2`))) (`KismetMathLibrary.Conv_BoolToInt` (`SceneComponent.IsAnySimulatingPhysics` (`self.Overhead_Light_3`)))) _trap_localinfluence_2)))))

(fn `UserConstructionScript`
  (set `PrimitiveComponent.bGenerateOverlapEvents` false (`self.Trigger`))
  (set `self.Active Timer` (`KismetMathLibrary.RandomFloatInRange` 1.0 2400.0)))