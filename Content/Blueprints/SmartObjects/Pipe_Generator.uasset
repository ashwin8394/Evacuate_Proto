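; Pipe generator actor that lays out a straight row of water pipe actors at construction time.
; The construction script adds one WaterPipe child actor component per NumPipes, evenly spaced along local X, and stores them in PipeObjects.
; Unconnected leftover logic builds spline mesh pipes along GenPath and tracks per-segment health, swapping in a broken mesh on damage.
; The event graph has no active behavior.
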(event `self.ReceiveTick`
  (params (DeltaSeconds :type "Float (single-precision)")))

(fn `UserConstructionScript`
  (`KismetArrayLibrary.Array_Clear` (`self.Pipe_Objects`))
  (for _index (range (`self.Num_Pipes`))
    (bind _returnvalue (`AddComponent|NODE_AddChildActorComponent-0` :`RelativeTransform` (`KismetMathLibrary.MakeTransform` (`KismetMathLibrary.MakeVector` (* _index 2400.0) 0.0 0.0))))
    (`ChildActorComponent.SetChildActorClass` _returnvalue "/Game/Blueprints/SmartObjects/WaterPipe.WaterPipe_C")
    (`SceneComponent.K2_AttachToComponent` _returnvalue (`self.DefaultSceneRoot`) "None" "KeepRelative" "KeepRelative" "KeepRelative" true)
    (`KismetArrayLibrary.Array_Add` (`self.Pipe_Objects`) _returnvalue)))