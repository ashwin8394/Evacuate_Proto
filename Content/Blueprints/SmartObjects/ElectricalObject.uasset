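; ElectricalObject is a smart object that, when fractured while electrically active, electrifies broken water pipes around it.
; On fracture it runs a large zero-length multi-sphere trace at its root and sets Electric on any hit WaterPipe that is already Broken.
; The trace then marks the object Broken, so Tick repeats it every frame while the object stays active, catching pipes that break later.
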(event `self.Object.OnComponentFracture`
  (params (HitPoint :type "Vector Structure (by ref)") (HitDirection :type "Vector Structure (by ref)"))
  (if (`self.Electrically Active`) :!label _label
    (`self.TraceForWater`)))

(event `self.ReceiveTick`
  (params (DeltaSeconds :type "Float (single-precision)"))
  (if (`self.Broken`)
    (goto _label)))

(fn `TraceForWater`
  (bind _returnvalue (`SceneComponent.K2_GetComponentLocation` (`self.DefaultSceneRoot`)))
  (bind _outhits (`KismetSystemLibrary.SphereTraceMultiForObjects` _returnvalue _returnvalue 4000.0 (`|MakeArray` "ObjectTypeQuery2" "ObjectTypeQuery1" :!type "EObjectTypeQuery Enum")))
  (`/Engine/EditorBlueprintResources/StandardMacros.DoOnce` false :!label _label
    (:`Completed`
      (for _array_element _outhits
        (bind (_bblockinghit _binitialoverlap _time _location _impactpoint _normal _impactnormal _physmat _hitactor) (`GameplayStatics.BreakHitResult` _array_element))
        (if (== (`GameplayStatics.GetObjectClass` _hitactor) "/Game/Blueprints/SmartObjects/WaterPipe.WaterPipe_C")
          (bind _aswater_pipe (cast `/Game/Blueprints/SmartObjects/WaterPipe` _hitactor))
          (if (`/Game/Blueprints/SmartObjects/WaterPipe.Broken` _aswater_pipe)
            (set `/Game/Blueprints/SmartObjects/WaterPipe.Electric` true _aswater_pipe))))
      (set `self.Broken` true)
      (goto _label :!via `Reset`))))

(fn `UserConstructionScript`)