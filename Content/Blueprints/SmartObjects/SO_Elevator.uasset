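; Interactive elevator that travels between an origin and an end target point when the player presses Interact.
; Overlap of the player pawn with ActivationTrigger opens or closes a gate on the input, so it only responds while the player is inside.
; Each press uses MoveComponentTo to ease the platform to the other point over a set time, reposition the trigger just above that point and flip AtOrigin.
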(event `self.ReceiveBeginPlay`
  (`self.EnableInput` (`GameplayStatics.GetPlayerController` 0)))

(event `InputAction|Interact`
  (params (Key :type "Key Structure" :default "AnyKey"))
  (bind _relativelocation (`SceneComponent.RelativeLocation` (`self.OriginTargetPoint`)))
  (bind _relativelocation_2 (`SceneComponent.RelativeLocation` (`self.EndTargetPoint`)))
  (:`Pressed`
    (`/Engine/EditorBlueprintResources/StandardMacros.Gate` true :!label _label
      (:`Exit`
        (if (`self.atOrigin`)
          (`KismetSystemLibrary.MoveComponentTo` (`self.elevator`) _relativelocation_2 (struct) true true (`self.Time`))
          (`KismetSystemLibrary.MoveComponentTo` (`self.ActivationTrigger`) (+ _relativelocation_2 (0.0 0.0 43.0)) (struct) false false 0.0)
          (set `self.atOrigin` false)
          (else
            (`KismetSystemLibrary.MoveComponentTo` (`self.elevator`) _relativelocation (struct) true true (`self.Time`))
            (`KismetSystemLibrary.MoveComponentTo` (`self.ActivationTrigger`) (+ _relativelocation (0.0 0.0 43.0)) (struct) false false 0.0)
            (set `self.atOrigin` true)))))))

(event `self.ActivationTrigger.OnComponentBeginOverlap`
  (params (OverlappedComponent :type "PrimitiveComponent Object Reference") (OtherActor :type "Actor Object Reference") (OtherComp :type "PrimitiveComponent Object Reference") (OtherBodyIndex :type Integer) (bFromSweep :type Boolean) (SweepResult :type "HitResult Structure (by ref)"))
  (if (== OtherActor (`GameplayStatics.GetPlayerPawn` 0))
    (goto _label :!via `Open`)))

(event `self.ActivationTrigger.OnComponentEndOverlap`
  (params (OverlappedComponent :type "PrimitiveComponent Object Reference") (OtherActor :type "Actor Object Reference") (OtherComp :type "PrimitiveComponent Object Reference") (OtherBodyIndex :type Integer))
  (if (== OtherActor (`GameplayStatics.GetPlayerPawn` 0))
    (goto _label :!via `Close`)))

(fn `UserConstructionScript`)