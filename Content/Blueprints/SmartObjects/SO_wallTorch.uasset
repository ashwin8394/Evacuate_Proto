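; Wall torch smart object that switches its fire effect and two point lights, and alters scene fog around it.
; Tick derives fire and light states from Active and EmitOnly, using paired DoOnce gates to apply changes only when needed.
; The construction script applies the same states in the editor.
; FogBurn overlaps drive a timeline that changes the first ExponentialHeightFog's start distance while the torch is active.
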(event `self.ReceiveBeginPlay`
  (bind _outactors (`GameplayStatics.GetAllActorsOfClass` "/Script/Engine.ExponentialHeightFog"))
  (set `self.Fog_Ref` (`KismetArrayLibrary.Array_Get` _outactors)))

(event `self.ReceiveTick`
  (params (DeltaSeconds :type "Float (single-precision)"))
  (bind _pointlight1 (`self.PointLight1`))
  (bind _active (`self.Active`))
  (bind _fire (`self.Fire`))
  (bind _pointlight (`self.PointLight`))
  (bind _emit (`self.emit`))
  (`|ExecutionSequence`
    (:`then_0`
      (if (!= (`self.emit`) (`self.Emit Light`))
        (set `self.emit` (`self.Emit Light`))
        (set `self.refresh` true)))
    (:`then_1`
      (if (`self.refresh`)
        (`|ExecutionSequence`
          (:`then_0`
            (goto _label :!via `Reset`))
          (:`then_1`
            (goto _label_2 :!via `Reset`))
          (:`then_2`
            _)))
      (if (`self.Inactive`)
        (`/Engine/EditorBlueprintResources/StandardMacros.DoOnce` false :!label _label
          (:`Completed`
            (`ActorComponent.SetActive` _fire false false)
            (`SceneComponent.SetVisibility` _pointlight false false)
            (`SceneComponent.SetVisibility` _pointlight1 false false)
            (set `self.refresh` false)
            (goto _label_2 :!via `Reset`)))
        (else
          (`/Engine/EditorBlueprintResources/StandardMacros.DoOnce` false :!label _label_2
            (:`Completed`
              (`ActorComponent.SetActive` _fire true false)
              (`SceneComponent.SetVisibility` _pointlight _emit false)
              (`SceneComponent.SetVisibility` _pointlight1 _emit false)
              (set `self.refresh` false)
              (goto _label :!via `Reset`))))))
    (:`then_2`
      (set `self.Inactive` (and (not _active) (not (`self.Emit Only`))))
      (set `self.Emit Light` _active))))

(event `self.FogBurn.OnComponentBeginOverlap`
  (params (OverlappedComponent :type "PrimitiveComponent Object Reference") (OtherActor :type "Actor Object Reference") (OtherComp :type "PrimitiveComponent Object Reference") (OtherBodyIndex :type Integer) (bFromSweep :type Boolean) (SweepResult :type "HitResult Structure (by ref)"))
  (bind (_direction _transition) (`Timeline|FogStartDist` :!via `Reverse` :!label _label_3)
    (:`Update`
      (if (`self.Active`)
        (`ExponentialHeightFogComponent.SetStartDistance` (`ExponentialHeightFog.Component` (`self.Fog_Ref`)) (* _transition 500.0))))))

(event `self.FogBurn.OnComponentEndOverlap`
  (params (OverlappedComponent :type "PrimitiveComponent Object Reference") (OtherActor :type "Actor Object Reference") (OtherComp :type "PrimitiveComponent Object Reference") (OtherBodyIndex :type Integer))
  (goto _label_3))

(fn `UserConstructionScript`
  (bind _output_get (set `self.emit` (`self.Emit Light`)))
  (`SceneComponent.SetVisibility` (`self.PointLight`) _output_get false)
  (`ActorComponent.SetActive` (`self.Fire`) (not (`self.Inactive`)) false)
  (`SceneComponent.SetVisibility` (`self.PointLight1`) _output_get false))