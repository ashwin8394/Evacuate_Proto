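; Large fire smart object that pairs a Fire effect component with a point light.
; Both follow the inverse of the Hidden flag, so the fire is active and the light visible only when not hidden.
; The construction script applies this state, and Tick reapplies it every frame by polling instead of reacting to changes.
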(event `self.ReceiveTick`
  (params (DeltaSeconds :type "Float (single-precision)"))
  (bind _returnvalue (not (`self.Hidden`)))
  (`ActorComponent.SetActive` (`self.Fire`) _returnvalue false)
  (`SceneComponent.SetVisibility` (`self.PointLight`) _returnvalue false))

(fn `UserConstructionScript`
  (bind _returnvalue (not (`self.Hidden`)))
  (`ActorComponent.SetActive` (`self.Fire`) _returnvalue false)
  (`SceneComponent.SetVisibility` (`self.PointLight`) _returnvalue false))