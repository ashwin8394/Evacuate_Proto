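; Breakable water pipe smart object that loses health when hit by actors other than the player or NPC classes, with a short cooldown between hits.
; At zero health it swaps to a broken mesh, shows water effects, then reveals a decal after a delay.
; Tick re-applies the health state and gradually grows the decal once broken.
; The construction script sets the intact or broken look from Health.
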(event `On Health Changed`
  (params (`New Health` :type "Float (double-precision)"))
  (bind _returnvalue (<= `New Health` 0.0))
  (if _returnvalue
    (set `self.Health` 0.0)
    (`StaticMeshComponent.SetStaticMesh` (`self.Pipe`) "/Game/Objects/Static/wall_pipe_Water_Pipe_Broken.wall_pipe_Water_Pipe_Broken")
    (`SceneComponent.SetVisibility` (`self.WaterBurst`) _returnvalue false)
    (`SceneComponent.SetVisibility` (`self.Water2`) _returnvalue false)
    (`SceneComponent.SetVisibility` (`self.WaterBack1`) _returnvalue false)
    (`KismetSystemLibrary.Delay` 0.75)
    (`SceneComponent.SetVisibility` (`self.Decal`) _returnvalue false)
    (set `self.Broken` true)
    (else
      (set `self.Health` `New Health`))))

(event `self.Pipe.OnComponentHit`
  (params (HitComponent :type "PrimitiveComponent Object Reference") (OtherActor :type "Actor Object Reference") (OtherComp :type "PrimitiveComponent Object Reference") (NormalImpulse :type "Vector Structure") (Hit :type "HitResult Structure (by ref)"))
  (bind _returnvalue (`GameplayStatics.GetObjectClass` OtherActor))
  (if (not (or (== _returnvalue "/Game/Objects/Character/Player_Character2.Player_Character2_C") (== _returnvalue "/Game/Blueprints/Character/AI_Character/NPC.NPC_C")))
    (`/Engine/EditorBlueprintResources/StandardMacros.DoOnce` false :!label _label
      (:`Completed`
        (`self.On Health Changed` (- (`self.Health`) 10.0))
        (`KismetSystemLibrary.Delay` 0.2)
        (goto _label :!via `Reset`)))))

(event `self.ReceiveTick`
  (params (DeltaSeconds :type "Float (single-precision)"))
  (bind _decal (`self.Decal`))
  (bind _returnvalue_x (`KismetMathLibrary.BreakVector` (`SceneComponent.K2_GetComponentScale` _decal)))
  (bind _returnvalue (+ _returnvalue_x 0.1))
  (`|ExecutionSequence`
    (:`then_0`
      (`self.On Health Changed` (`self.Health`))
      (if (`self.Broken`)
        (`|ExecutionSequence`
          (:`then_0`
            (if (< _returnvalue_x 1.5)
              (`/Engine/EditorBlueprintResources/StandardMacros.DoOnce` false :!label _label_2
                (:`Completed`
                  (`KismetSystemLibrary.Delay` 0.05)
                  (`SceneComponent.SetWorldScale3D` _decal (`KismetMathLibrary.MakeVector` _returnvalue _returnvalue 1.0))
                  (goto _label_2 :!via `Reset`))))))))))

(fn `UserConstructionScript`
  (bind _pipe (`self.Pipe`))
  (bind _returnvalue (<= (`self.Health`) 0.0))
  (if _returnvalue
    (`StaticMeshComponent.SetStaticMesh` _pipe "/Game/Objects/Static/wall_pipe_Water_Pipe_Broken.wall_pipe_Water_Pipe_Broken")
    (else
      (`StaticMeshComponent.SetStaticMesh` _pipe "/Game/Objects/Static/wall_pipe_Water_Pipe.wall_pipe_Water_Pipe")))
  (`SceneComponent.SetVisibility` (`self.WaterBurst`) _returnvalue false)
  (`SceneComponent.SetVisibility` (`self.Water2`) _returnvalue false)
  (`SceneComponent.SetVisibility` (`self.WaterBack1`) _returnvalue false)
  (`SceneComponent.SetVisibility` (`self.Decal`) _returnvalue false))