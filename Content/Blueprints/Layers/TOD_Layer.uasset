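; Time-of-day layer Blueprint that switches the level's TOD_Light actors between day and night states.
; BeginPlay gathers every TOD_Light into emit-only and non-emit lists, which the day and night events treat alike.
; isNight activates all lights, while isDay deactivates those not flagged Exclude.
; A separate CalcTime helper converts sun position to a 24-hour value, mirrored when SunZ is negative.
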(event `self.ReceiveBeginPlay`
  (`KismetArrayLibrary.Array_Clear` (`self.Emit List`))
  (`KismetArrayLibrary.Array_Clear` (`self.Non-Emit_List`))
  (bind _outactors (`GameplayStatics.GetAllActorsOfClass` "/Game/Blueprints/DataTypes/TOD_Light.TOD_Light_C"))
  (for _array_element _outactors
    (if (`/Game/Blueprints/DataTypes/TOD_Light.Emit Only` _array_element)
      (`KismetArrayLibrary.Array_Add` (`self.Emit List`) _array_element)
      (else
        (`KismetArrayLibrary.Array_Add` (`self.Non-Emit_List`) _array_element)))))

(event `isNight`
  (for _array_element (`self.Emit List`)
    (set `/Game/Blueprints/DataTypes/TOD_Light.Active` true _array_element))
  (for _array_element_2 (`self.Non-Emit_List`)
    (set `/Game/Blueprints/DataTypes/TOD_Light.Active` true _array_element_2)))

(event `isDay`
  (for _array_element (`self.Emit List`)
    (if (not (`/Game/Blueprints/DataTypes/TOD_Light.Exclude` _array_element))
      (set `/Game/Blueprints/DataTypes/TOD_Light.Active` false _array_element)))
  (for _array_element_2 (`self.Non-Emit_List`)
    (if (not (`/Game/Blueprints/DataTypes/TOD_Light.Exclude` _array_element_2))
      (set `/Game/Blueprints/DataTypes/TOD_Light.Active` false _array_element_2))))

(fn `calcTime`
  (params (SunPos :type "Float (double-precision)") (SunZ :type "Float (double-precision)"))
  (returns (TotalHours :type "Float (double-precision)"))
  (locals (Hours :type "Float (double-precision)"))
  (bind _returnvalue (/ (* 24 (+ SunPos 90.0)) 180.0))
  (if (< SunZ 0.0)
    (return (- 24.0 _returnvalue))
    (else
      (return _returnvalue))))

(fn `UserConstructionScript`
  (`KismetArrayLibrary.Array_Clear` (`self.Emit List`))
  (`KismetArrayLibrary.Array_Clear` (`self.Non-Emit_List`)))