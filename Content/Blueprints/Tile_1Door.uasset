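; Tile_1Door is a level tile with a single exit that registers itself as the current tile of NPCs entering it.
; Its construction script rebuilds the ExitPoints list from the world location of the Exit component.
; When an actor of class NPC begins overlapping TileBounds, the tile sets itself as CurrentTile on that NPC's NPC_Controller.
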(event `self.TileBounds.OnComponentBeginOverlap`
  (params (OverlappedComponent :type "PrimitiveComponent Object Reference") (OtherActor :type "Actor Object Reference") (OtherComp :type "PrimitiveComponent Object Reference") (OtherBodyIndex :type Integer) (bFromSweep :type Boolean) (SweepResult :type "HitResult Structure (by ref)"))
  (if (== (`GameplayStatics.GetObjectClass` OtherActor) "/Game/Blueprints/Character/AI_Character/NPC.NPC_C")
    (bind _asnpc (cast `/Game/Blueprints/Character/AI_Character/NPC` OtherActor))
    (bind _returnvalue (`AIBlueprintHelperLibrary.GetAIController` _asnpc))
    (bind _asnpc_controller (cast `/Game/Blueprints/Character/AI_Character/NPC_Controller` _returnvalue))
    (set `/Game/Blueprints/Character/AI_Character/NPC_Controller.CurrentTile` self _asnpc_controller)))

(fn `UserConstructionScript`
  (bind _exitpoints (`self.ExitPoints`))
  (`KismetArrayLibrary.Array_Clear` _exitpoints)
  (`KismetArrayLibrary.Array_Add` _exitpoints (`SceneComponent.K2_GetComponentLocation` (`self.exit`))))